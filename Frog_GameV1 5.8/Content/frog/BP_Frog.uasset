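; Player frog character with a mouse-aimed charge jump, wall stick and wall jump, plus HUD pause and lives-based game over.
; Tick builds charge while jump is held, draws a debug-line arc in the YZ plane, sphere-traces for walls and regenerates stamina.
; Releasing jump launches the frog, or kicks it off a stuck wall, where gravity is suspended for a limited time.
; Tongue logic is disconnected, and JumpStamCost is never called here.
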(event Custom|CheckForWall
  (bind _returnvalue (Transformation|GetActorLocation))
  (bind _returnvalue_2 (Transformation|GetActorLocation))
  (bind _outhit (Collision|SphereTraceByChannel _returnvalue_2 (+ _returnvalue_2 6e+01) 35.0 "TraceTypeQuery2" false 0 "None"))
  (if (.bBlockingHit (Collision|BreakHitResult _outhit))
    (Variables|Default|SetWallDetected true)
    (Variables|Default|SetWallNormal (.ImpactNormal (Collision|BreakHitResult _outhit)))
    (else
      (bind _outhit_2 (Collision|SphereTraceByChannel _returnvalue (+ _returnvalue -6e+01) 35.0 "TraceTypeQuery2" false 0 "None"))
      (Variables|Default|SetWallDetected true)
      (Variables|Default|SetWallNormal (.ImpactNormal (Collision|BreakHitResult _outhit_2))))))

(event Custom|TryWallStick
  (if (not (Variables|Default|GetIs%20Stickingto%20Wall?))
    (if (Variables|Default|GetCan%20Stickto%20Wall?)
      (if (Variables|Default|GetWallDetected)
        (if (not (AI|Components|NavMovement|IsMovingonGround (Variables|Character|GetCharacterMovement)))
          (Variables|Default|SetIs%20Stickingto%20Wall? true)
          (if (AI|Components|NavMovement|IsFalling (Variables|Character|GetCharacterMovement))
            (Components|Movement|StopMovementImmediately (Variables|Character|GetCharacterMovement))
            (Variables|/Script/Engine.CharacterMovementComponent|SetGravityScale (Variables|Character|GetCharacterMovement) 0.0)
            (Utilities|FlowControl|Delay (Variables|Default|GetWallStickTime))
            (CallFunction|EndWallStick)))))))

(event Custom|EndWallStick
  (Variables|Default|SetIs%20Stickingto%20Wall? false)
  (Variables|/Script/Engine.CharacterMovementComponent|SetGravityScale (Variables|Character|GetCharacterMovement) (Variables|Default|GetNormalGravityScale))
  (Variables|Default|SetCan%20Stickto%20Wall? false))

(event Input|EnhancedActionEvents|EnhancedInputActionIA_TongueShoot
  (params (ActionValue :type Boolean) (ElapsedSeconds :type Float%20%28double-precision%29) (TriggeredSeconds :type Float%20%28double-precision%29) (InputAction :type Input%20Action%20Object%20Reference :default "/Game/frog/InputAction/IA_TongueShoot.IA_TongueShoot")))

(event Input|EnhancedActionEvents|EnhancedInputActionIA_Jump
  (params (ActionValue :type Boolean) (ElapsedSeconds :type Float%20%28double-precision%29) (TriggeredSeconds :type Float%20%28double-precision%29) (InputAction :type Input%20Action%20Object%20Reference :default "/Game/Input/Actions/IA_Jump.IA_Jump"))
  (:Started
    (if (not (<= (Variables|Default|GetCurrentStamina) 0.0))
      (if (not (Variables|Default|GetCan%20Stickto%20Wall?))
        (if (Variables|Default|Getjump?)
          (if (AI|Components|NavMovement|IsMovingonGround (Variables|Character|GetCharacterMovement))
            ;[0.15 0.15 0.15 0.5] If player starts holding the jump button reset amount to 0
            (Variables|Default|SetIsChargingJump true)
            (Variables|Default|SetJumpChargeAmount 0.0))))))
  (:Completed
    ;[0.15 0.15 0.15 0.5] If the player is jumping
    (if (Variables|Default|GetIsChargingJump)
      (if (Variables|Default|GetIs%20Stickingto%20Wall?)
        (Variables|Default|SetIs%20Stickingto%20Wall? false)
        (Variables|/Script/Engine.CharacterMovementComponent|SetGravityScale (Variables|Character|GetCharacterMovement) (Variables|Default|GetNormalGravityScale))
        (Character|LaunchCharacter (+ (* (Variables|Default|GetWallNormal) (Variables|Default|GetWallJumpAwayForce)) (Math|Vector|MakeVector 0.0 0.0 (Variables|Default|GetWallJumpUpForce))) true true)
        (Variables|Default|SetCan%20Stickto%20Wall? false)
        (else
          ;[0.15 0.15 0.15 0.5] Use the result from the multiplication as the launch velocity and what direction the character should be launched in - Set charging jump back to false when completed
          (Character|LaunchCharacter (* (Variables|Default|GetJumpDirection) (Math|Float|Lerp (Variables|Default|GetMinJumpStrength) (Variables|Default|GetMaxJumpStrenght) (/ (Variables|Default|GetJumpChargeAmount) (Variables|Default|GetJumpChargeMax)))) false false)
          (Utilities|FlowControl|Delay (Variables|Default|Getcooldown))
          (Variables|Default|SetIsChargingJump false))))))

(event EventBeginPlay
  (Input|AddMappingContext (PlayerController|LocalPlayerSubsystems|GetEnhancedInputLocalPlayerSubsystem (Game|GetPlayerController 0)) "/Game/frog/InputAction/IMC_Frog.IMC_Frog" 0 "(bIgnoreAllPressedKeysUntilRelease=True,bForceImmediately=False,bNotifyUserSettings=False)")
  (Variables|/Script/Engine.PlayerController|SetbShowMouseCursor (Game|GetPlayerController 0) true)
  ;[0.15 0.15 0.15 0.5] Add HUD to Viewport
  (bind _returnvalue (UserInterface|CreateWidget "/Game/UI/WB_HUD.WB_HUD_C"))
  (bind _output_get (Variables|Default|SetHUD _returnvalue))
  (UserInterface|Viewport|AddtoViewport _output_get 0))

(event Collision|EventActorBeginOverlap
  (params (OtherActor :type Actor%20Object%20Reference)))

(event EventTick
  (params (DeltaSeconds :type Float%20%28single-precision%29))
  ;[0.15 0.15 0.15 0.5] Continually checks if Jump has been triggered
  (if (Variables|Default|GetIsChargingJump)
    ;[0.15 0.15 0.15 0.5] Calculate the length of time jump has been held + max charge amount * secs -> clamp value so its no more than the max jump amount allowed
    (Variables|Default|SetJumpChargeAmount (Math|Float|Clamp(Float) (+ (Variables|Default|GetJumpChargeAmount) (* (Variables|Default|GetJumpChargeMax) DeltaSeconds)) 0.0 (Variables|Default|GetJumpChargeMax)))
    ;[0.15 0.15 0.15 0.5] Divide the charge amount by the max to get a % set that as charge percent - lerp node finds the Jump strength by calculating where the strength falls by through the percentage
    (bind _output_get (Variables|Default|SetCharge%20Percent (/ (Variables|Default|GetJumpChargeAmount) (Variables|Default|GetJumpChargeMax))))
    (Variables|Default|SetJumpstrength (Math|Float|Lerp (Variables|Default|GetMinJumpStrength) (Variables|Default|GetMaxJumpStrenght) _output_get))
    (bind _jumpdirection (CallFunction|JumpAim))
    ;[0.15 0.15 0.15 0.5] Jump Direction + strength are multiplied to predict the velocity of the jump and a prediction line in developed based on this
    (bind _output_get_2 (Variables|Default|SetJumpDirection _jumpdirection))
    (bind _output_get_3 (Variables|Default|SetPreviewVelocity (* _output_get_2 (Variables|Default|GetJumpstrength))))
    (CallFunction|DrawJumpPrediction (Transformation|GetActorLocation) _output_get_3)
    (if (not (Variables|Default|GetIs%20Stickingto%20Wall?))
      (CallFunction|CheckforWall)
      (CallFunction|TryWallStick)
      (if (not (Variables|Default|GetIsConsumingStam))
        (CallFunction|StamRegen DeltaSeconds)))))

(event Input|KeyboardEvents|P
  (params (Key :type Key%20Structure))
  (bind _returnvalue (Game|GetPlayerController 0))
  ;[0.15 0.15 0.15 0.5] HUD
  ;;[0.15 0.15 0.15 0.5] Pause Screen Button
  (:Pressed
    (Variables|/Script/UMG.Widget|SetVisibility (Variables|/Game/UI/WB_HUD.WB_HUD_C|GetPause_Screen (Variables|Default|GetHUD)) "Visible")
    (Variables|/Script/Engine.PlayerController|SetbShowMouseCursor _returnvalue true)
    (Game|SetGamePaused true)
    (Input|SetInputModeUIOnly _returnvalue 0 "DoNotLock" false)))

(fn ConstructionScript)

(fn DrawJumpPrediction
  (params (StartLocation :type Vector) (LaunchVelocity :type Vector))
  (LocalVariables|SetPreviousPoint StartLocation)
  (for _index (range 0 20)
    (LocalVariables|SetTime (* _index 0.05))
    (bind _output_get (LocalVariables|SetGravity%20Displacement (* (* (Components|Movement|GetGravityZ (Variables|Character|GetCharacterMovement)) (* (LocalVariables|GetTime) (LocalVariables|GetTime))) 0.5)))
    (bind _output_get_2 (LocalVariables|SetGravity%20vector (Math|Vector|MakeVector 0.0 0.0 _output_get)))
    (LocalVariables|SetCurrentpoint (+ _output_get_2 (+ (* LaunchVelocity (LocalVariables|GetTime)) StartLocation)))
    (Rendering|Debug|DrawDebugLine (LocalVariables|GetPreviousPoint) (LocalVariables|GetCurrentpoint) "(R=1.000000,G=1.000000,B=1.000000,A=1.000000)" 0.0 5.0)
    (LocalVariables|SetPreviousPoint (LocalVariables|GetCurrentpoint))))

(fn JumpAim
  (bind _returnvalue (Game|GetPlayerController 0))
  (bind (_locationx _locationy) (Game|Player|GetMousePosition _returnvalue))
  (bind (_worldposition _worlddirection) (Class|GameplayStatics|DeprojectScreentoWorld _returnvalue (Math|Vector2D|MakeVector2D _locationx _locationy)))
  (bind _output_get (Variables|Default|SetRayStart _worldposition))
  (bind _output_get_2 (Variables|Default|SetRayDiirection _worlddirection))
  (bind _output_get_3 (Variables|Default|SetMouse%20world%20position (+ (* _output_get_2 (- (- 0.0 (.Y (Math|Vector|BreakVector _output_get))) (.Y (Math|Vector|BreakVector _output_get_2)))) _output_get)))
  (return (Math|Vector|Normalize (Math|Vector|MakeVector 0.0 (.Y (Math|Vector|BreakVector (- _output_get_3 (Transformation|GetActorLocation)))) (.Z (Math|Vector|BreakVector (- _output_get_3 (Transformation|GetActorLocation))))))))

(fn TakeDamage
  (params (Damage :type Integer))
  (bind _output_get (Variables|Default|SetLives (- (Variables|Default|GetLives) Damage)))
  (if (== _output_get 0)
    (Widget|SetVisibility (Variables|Default|GetHUD) "Visible")
    (CallFunction|DeathOperations)))

(fn DeathOperations
  (bind _returnvalue (Game|GetPlayerController 0))
  (Game|SetGamePaused true)
  (Variables|/Script/Engine.PlayerController|SetbShowMouseCursor _returnvalue true)
  (Input|SetInputModeUIOnly _returnvalue 0 "DoNotLock" false)
  (Widget|SetVisibility (Variables|/Game/UI/WB_HUD.WB_HUD_C|GetGameOver_Screen (Variables|Default|GetHUD)) "Visible"))

(fn JumpStamCost
  (Variables|Default|SetIsConsumingStam true)
  (Variables|Default|SetCurrentStamina (- (Variables|Default|GetCurrentStamina) (Variables|Default|GetJumpCost)))
  (Variables|Default|SetIsConsumingStam false))

(fn StamRegen
  (params (Dseconds :type Float%20%28double-precision%29))
  (if (< (Variables|Default|GetCurrentStamina) (Variables|Default|GetMaxStamina))
    (Variables|Default|SetCurrentStamina (Math|Float|Clamp(Float) (+ (Variables|Default|GetCurrentStamina) (* (Variables|Default|GetStamRegenRate) Dseconds)) 0.0 (Variables|Default|GetMaxStamina)))))