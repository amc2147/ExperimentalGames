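; BP_Flies is a pickup actor that grants extra lives to the player's frog in a frog game.
; When a BP_Frog overlaps its Box, it adds LivestoAdd to the frog's Lives and refreshes the HUD, but only if the frog has fewer than five lives.
; The pickup destroys itself on any frog overlap, even when no lives are added.
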(event OnComponentBeginOverlap(Box)
  (params (OverlappedComponent :type Primitive%20Component%20Object%20Reference) (OtherActor :type Actor%20Object%20Reference) (OtherComp :type Primitive%20Component%20Object%20Reference) (OtherBodyIndex :type Integer) (bFromSweep :type Boolean) (SweepResult :type Hit%20Result%20Structure%20%28by%20ref%29))
  (bind _asbp_frog (Utilities|Casting|CastToBP_Frog OtherActor))
  (if (>= (Variables|/Game/frog/BP_Frog.BP_Frog_C|GetLives _asbp_frog) 5)
    (Actor|DestroyActor)
    (else
      (Variables|/Game/frog/BP_Frog.BP_Frog_C|SetLives _asbp_frog (+ (Variables|/Game/frog/BP_Frog.BP_Frog_C|GetLives _asbp_frog) (Variables|Default|GetLivestoAdd)))
      (Default|UpdateLives (Variables|/Game/frog/BP_Frog.BP_Frog_C|GetHUD _asbp_frog))
      (Actor|DestroyActor))))

(event EventBeginPlay)

(event Collision|EventActorBeginOverlap
  (params (OtherActor :type Actor%20Object%20Reference)))

(event EventTick
  (params (DeltaSeconds :type Float%20%28single-precision%29)))

(fn ConstructionScript)