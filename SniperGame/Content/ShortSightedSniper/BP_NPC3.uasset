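; BP_NPC3 is an NPC target in ShortSightedSniper whose death ends the level.
; DamageAI feeds UpdateHealth, which at zero health calls a montage play and runs DeathOperations.
; With a valid AI controller, DeathOperations stops its logic, disables capsule collision, unpossesses and triggers Death.
; After a short delay, Death destroys the actor, shows the HUD's GameOverScreen as level-complete screen, enables the cursor and plays a sound.
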(event Custom|Death
  (bind _returnvalue (Game|GetPlayerController 0))
  (Utilities|FlowControl|Delay 0.5)
  (Actor|DestroyActor)
  ;[0.15 0.15 0.15 0.5] Adding Level Complete Screen when Target Shot
  (bind _returnvalue_2 (UserInterface|CreateWidget "/Game/UI/WB_PlayerHUD.WB_PlayerHUD_C"))
  (bind _output_get (Variables|Default|SetPlayerHUD _returnvalue_2))
  (UserInterface|Viewport|AddtoViewport _output_get 0)
  (Widget|SetVisibility (Variables|/Game/UI/WB_PlayerHUD.WB_PlayerHUD_C|GetGameOverScreen (Variables|Default|GetPlayerHUD)) "Visible")
  (Variables|/Script/Engine.PlayerController|SetbShowMouseCursor _returnvalue true)
  (Input|SetInputModeGameandUI _returnvalue 0 "DoNotLock" true false)
  (Audio|PlaySound2D "/Game/ShortSightedSniper/GameFeel/SoundEffects/UISFX/Laser_2.Laser_2" 1.0 1.0 0.0 0 0))

(event EventBeginPlay)

(event Collision|EventActorBeginOverlap
  (params (OtherActor :type Actor%20Object%20Reference)))

(event EventTick
  (params (DeltaSeconds :type Float%20%28single-precision%29)))

(event EventDamageAI
  (params (Damage :type Float%20%28double-precision%29))
  (CallFunction|UpdateHealth Damage)
  (Development|PrintString "Hello"))

(fn ConstructionScript)

(fn DeathOperations
  (bind _self self)
  (bind _returnvalue (AI|GetAIController _self))
  (Utilities|IsValid _returnvalue
    (:Is%20Valid
      (AI|Logic|StopLogic (Variables|/Script/AIModule.AIController|GetBrainComponent _returnvalue) "")
      (Collision|SetCollisionEnabled (Variables|Collision|GetCapsuleComponent) "NoCollision")
      (Actor|SetLifeSpan _returnvalue 0.1)
      (Pawn|UnPossess _returnvalue)
      (CallFunction|Death))))

(fn UpdateHealth
  (params (Damage :type Float%20%28double-precision%29))
  (Variables|Default|SetCurrentHealth (- (Variables|Default|GetCurrentHealth) Damage))
  (if (<= (Variables|Default|GetCurrentHealth) 0.0)
    (Variables|Default|SetIsDead true)
    (Animation|PlayAnimMontage 0 1.0 "None")
    (CallFunction|DeathOperations)))