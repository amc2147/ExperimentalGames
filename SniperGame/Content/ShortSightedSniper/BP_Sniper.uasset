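; BP_Sniper is a sniper weapon Blueprint built around a ScopeCapture component for its scope view.
; SetScopeActive switches that component's tick on or off from the requested state, but always sets its visibility to false.
; Two getters expose the component's world location and rotation as the scope viewpoint.
; The event graph and construction script contain no logic.
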(event EventBeginPlay)

(event Collision|EventActorBeginOverlap
  (params (OtherActor :type Actor%20Object%20Reference)))

(event EventTick
  (params (DeltaSeconds :type Float%20%28single-precision%29)))

(fn ConstructionScript)

(fn SetScopeActive
  (params (NewActiveState :type Boolean))
  (bind _scopecapture (Variables|Default|GetScopeCapture))
  (Rendering|SetVisibility _scopecapture false false)
  (Components|Tick|SetComponentTickEnabled _scopecapture NewActiveState))

(fn GetScopeViewlocation
  (return (Transformation|GetWorldLocation (Variables|Default|GetScopeCapture))))

(fn GetScopeViewRotation
  (return (Transformation|GetWorldRotation (Variables|Default|GetScopeCapture))))