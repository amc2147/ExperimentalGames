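; BP_MainNPC is an AI-controlled NPC character that takes damage and can die.
; On BeginPlay it picks a random skeletal mesh from NPCmeshs for visual variety.
; DamageAI feeds UpdateHealth, which subtracts health and, at zero or below, sets IsDead, calls PlayAnimMontage and runs DeathOperations.
; DeathOperations stops the AI brain, disables capsule collision, then unpossesses and expires the controller.
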(event OnComponentBeginOverlap(Box)
  (params (OverlappedComponent :type Primitive%20Component%20Object%20Reference) (OtherActor :type Actor%20Object%20Reference) (OtherComp :type Primitive%20Component%20Object%20Reference) (OtherBodyIndex :type Integer) (bFromSweep :type Boolean) (SweepResult :type Hit%20Result%20Structure%20%28by%20ref%29)))

(event EventBeginPlay
  (Components|SkeletalMesh|SetSkeletalMeshAsset (Variables|Character|GetMesh) (.OutItem (Utilities|Array|Random (Variables|Default|GetNPCmeshs)))))

(event Collision|EventActorBeginOverlap
  (params (OtherActor :type Actor%20Object%20Reference)))

(event EventTick
  (params (DeltaSeconds :type Float%20%28single-precision%29)))

(event EventDamageAI
  (params (Damage :type Float%20%28double-precision%29))
  (CallFunction|UpdateHealth Damage))

(fn ConstructionScript)

(fn DeathOperations
  (bind _self self)
  (bind _returnvalue (AI|GetAIController _self))
  (Utilities|IsValid _returnvalue
    (:Is%20Valid
      (AI|Logic|StopLogic (Variables|/Script/AIModule.AIController|GetBrainComponent _returnvalue) "")
      (Collision|SetCollisionEnabled (Variables|Collision|GetCapsuleComponent) "NoCollision")
      (Actor|SetLifeSpan _returnvalue 0.1)
      (Pawn|UnPossess _returnvalue))))

(fn UpdateHealth
  (params (Damage :type Float%20%28double-precision%29))
  (Variables|Default|SetCurrentHealth (- (Variables|Default|GetCurrentHealth) Damage))
  (if (<= (Variables|Default|GetCurrentHealth) 0.0)
    (Variables|Default|SetIsDead true)
    (Animation|PlayAnimMontage 0 1.0 "None")
    (CallFunction|DeathOperations)))